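; An affordance Blueprint that shows or hides a set of actors when it is interacted with.
; Its Interact override calls the parent, flips the CurrentlyVisible flag and applies it to the root component of each actor in ActorsToToggle.
; The visibility change does not propagate to child components, and BeginPlay and Tick are unused.
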(event EventBeginPlay
  (|CallParentFunction) ; This node is disabled and will not be called.\nDrag off pins to build functionality.
)

(event EventTick
  (params (DeltaSeconds :type Float%20%28single-precision%29))
  (|CallParentFunction DeltaSeconds) ; This node is disabled and will not be called.\nDrag off pins to build functionality.
)

(fn Interact
  (|CallParentFunction)
  (Variables|Default|Setcurrently_visible (not (Variables|Default|Getcurrently_visible)))
  (for _array_element (Variables|Default|Getactors_to_toggle)
    (Rendering|SetVisibility (Variables|/Script/Engine.Actor|GetRootComponent _array_element) (Variables|Default|Getcurrently_visible) false)))