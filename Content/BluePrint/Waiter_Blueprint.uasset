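; Waiter actor that shows its text render when the player comes close and hides it otherwise.
; Every Tick it measures the distance to player pawn 0 and toggles the text's hidden-in-game state against a fixed range threshold, with no overlap events involved.
; It also prints that distance to the screen each frame as debug output.
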(event EventBeginPlay)

(event Collision|EventActorBeginOverlap
  (params (OtherActor :type Actor%20Object%20Reference)))

(event EventTick
  (params (DeltaSeconds :type Float%20%28single-precision%29))
  (bind _returnvalue (Game|Player|GetPlayerPawn 0))
  (bind _self self)
  (bind _returnvalue_2 (Transformation|GetDistanceTo _returnvalue _self))
  (Development|PrintString (Utilities|String|ToString(Float) _returnvalue_2))
  (if (< _returnvalue_2 5e+02)
    (Development|SetHiddeninGame (Variables|Default|GetTextRender) false false)
    (else
      (Development|SetHiddeninGame (Variables|Default|GetTextRender) true false))))

(fn ConstructionScript)