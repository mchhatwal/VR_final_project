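; BP_Apple is an apple actor that can be sliced with a knife or sold in a sell box, driven by its Hit event.
; A hit from BP_Knife plays a crack sound, spawns four sliced-apple actors at one offset from the apple, then destroys it.
; A hit from the sell box increments AppleNum on every shop manager found via GetAllActorsOfClass, then destroys the apple.
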(event EventBeginPlay)

(event Collision|EventActorBeginOverlap
  (params (OtherActor :type Actor%20Object%20Reference)))

(event EventTick
  (params (DeltaSeconds :type Float%20%28single-precision%29)))

(event Collision|EventHit
  (params (MyComp :type Primitive%20Component%20Object%20Reference) (Other :type Actor%20Object%20Reference) (OtherComp :type Primitive%20Component%20Object%20Reference) (bSelfMoved :type Boolean) (HitLocation :type Vector :default "0, 0, 0") (HitNormal :type Vector :default "0, 0, 0") (NormalImpulse :type Vector :default "0, 0, 0") (Hit :type Hit%20Result%20Structure%20%28by%20ref%29))
  (bind _returnvalue (Utilities|GetClass Other))
  (bind _returnvalue_2 (Transformation|GetActorLocation))
  (bind _returnvalue_3 (+ _returnvalue_2 "40.000000,0,0"))
  (Development|PrintString (Utilities|String|ToString(Object) Other) false)
  (if (== _returnvalue "/Game/Blueprints/BP_Knife.BP_Knife_C")
    (Audio|PlaySoundatLocation "/Game/Audios/apple-crack.apple-crack" HitLocation "0, 0, 0" 2e+01 0.0 0.12 0 0 0 0)
    (Game|SpawnActorfromClass "/Game/Blueprints/Sliced_Apple_Blueprint.Sliced_Apple_Blueprint_C" (Math|Transform|MakeTransform _returnvalue_3 "0, 0, 0" "1.000000,1.000000,1.000000") "AlwaysSpawn" 0 0)
    (Game|SpawnActorfromClass "/Game/Blueprints/Sliced_Apple_Blueprint.Sliced_Apple_Blueprint_C" (Math|Transform|MakeTransform _returnvalue_3 "0, 0, 0" "1.000000,1.000000,1.000000") "AlwaysSpawn" 0 0)
    (Game|SpawnActorfromClass "/Game/Blueprints/Sliced_Apple_Blueprint.Sliced_Apple_Blueprint_C" (Math|Transform|MakeTransform _returnvalue_3 "0, 0, 0" "1.000000,1.000000,1.000000") "AlwaysSpawn" 0 0)
    (Game|SpawnActorfromClass "/Game/Blueprints/Sliced_Apple_Blueprint.Sliced_Apple_Blueprint_C" (Math|Transform|MakeTransform _returnvalue_3 "0, 0, 0" "1.000000,1.000000,1.000000") "AlwaysSpawn" 0 0)
    (Actor|DestroyActor)
    (elif (== _returnvalue "/Game/Blueprints/sellbox_Blueprint.sellbox_Blueprint_C")
      (bind _outactors (Actor|GetAllActorsOfClass "/Game/Blueprints/shop_manager_Blueprint.shop_manager_Blueprint_C"))
      (for _array_element _outactors
        (Variables|/Game/Blueprints/shop_manager_Blueprint.shop_manager_Blueprint_C|Setapple_num _array_element (+ (Variables|/Game/Blueprints/shop_manager_Blueprint.shop_manager_Blueprint_C|Getapple_num _array_element) 1)))
      (Actor|DestroyActor))))

(fn ConstructionScript)