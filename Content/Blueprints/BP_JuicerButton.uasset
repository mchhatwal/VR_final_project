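; BP_JuicerButton is a toggle button that switches the juicer on and off to turn carrots into carrot juice.
; Each Box overlap flips JuicerOn and teleports the button between its starting position and a lowered pressed one.
; While on, Tick looks up BP_Juicer and, if its CarrotIn flag is set, destroys the carrot and spawns a tiny BP_CarrotJuice at a hardcoded world transform.
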(event OnComponentBeginOverlap(Box)
  (params (OverlappedComponent :type Primitive%20Component%20Object%20Reference) (OtherActor :type Actor%20Object%20Reference) (OtherComp :type Primitive%20Component%20Object%20Reference) (OtherBodyIndex :type Integer) (bFromSweep :type Boolean) (SweepResult :type Hit%20Result%20Structure%20%28by%20ref%29))
  (if (not (Variables|Default|GetJuicerOn))
    (Transformation|SetActorTransform (Variables|Default|GetIn_Position) false true)
    (Variables|Default|SetJuicerOn true)
    (else
      (Transformation|SetActorTransform (Variables|Default|GetOut_Position) false true)
      (Variables|Default|SetJuicerOn false))))

(event EventBeginPlay
  (bind _returnvalue (Transformation|GetActorTransform))
  (Variables|Default|SetOut_Position (Math|Transform|MakeTransform (.location _returnvalue) (.rotation _returnvalue) (.scale _returnvalue)))
  (Variables|Default|SetIn_Position (Math|Transform|MakeTransform (- (.location _returnvalue) "0.000000,0.000000,10.000000") (.rotation _returnvalue) (.scale _returnvalue)))
  (Input|EnableInput (Game|GetPlayerController 0)))

(event EventTick
  (params (DeltaSeconds :type Float%20%28single-precision%29))
  (if (Variables|Default|GetJuicerOn)
    (bind _returnvalue (Actor|GetActorOfClass "/Game/BP_Juicer.BP_Juicer_C"))
    (if (Variables|/Game/BP_Juicer.BP_Juicer_C|GetCarrotIn _returnvalue)
      (Actor|DestroyActor (Variables|/Game/BP_Juicer.BP_Juicer_C|GetCarrot _returnvalue))
      (Game|SpawnActorfromClass "/Game/OutsideResource/Juice--f9zLzhRRkZg/BP_CarrotJuice.BP_CarrotJuice_C" (Math|Transform|MakeTransform "750.000000,-376.000000,42.000000" "0, 0,90.000000" "0.000100,0.000100,0.000100") "AlwaysSpawn" 0 0))))

(fn ConstructionScript)