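; A pressable button actor that toggles the GasOn flag on the RestaurantGameState.
; At BeginPlay it stores its starting transform as the out position and one 10 units lower as the in position.
; Each begin overlap on its Box component flips the flag, then teleports the actor to the pressed or raised transform to match.
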(event OnComponentBeginOverlap(Box)
  (params (OverlappedComponent :type Primitive%20Component%20Object%20Reference) (OtherActor :type Actor%20Object%20Reference) (OtherComp :type Primitive%20Component%20Object%20Reference) (OtherBodyIndex :type Integer) (bFromSweep :type Boolean) (SweepResult :type Hit%20Result%20Structure%20%28by%20ref%29))
  (Development|PrintString (Utilities|GetDisplayName OverlappedComponent) false true "(R=0.000000,G=0.660000,B=1.000000,A=1.000000)" 2e+01)
  (bind _asrestaurant_game_state (Utilities|Casting|CastToRestaurantGameState (Game|GetGameState)))
  (Variables|/Game/Blueprints/RestaurantGameState.RestaurantGameState_C|SetGas_On _asrestaurant_game_state (not (Variables|/Game/Blueprints/RestaurantGameState.RestaurantGameState_C|GetGas_On _asrestaurant_game_state)))
  (if (Variables|/Game/Blueprints/RestaurantGameState.RestaurantGameState_C|GetGas_On _asrestaurant_game_state)
    (Transformation|SetActorTransform (Variables|Default|GetIn_Position) false true)
    (else
      (Transformation|SetActorTransform (Variables|Default|GetOut_Position) false true))))

(event EventBeginPlay
  (bind _returnvalue (Transformation|GetActorTransform))
  (Variables|Default|SetOut_Position (Math|Transform|MakeTransform (.location _returnvalue) (.rotation _returnvalue) (.scale _returnvalue)))
  (Variables|Default|SetIn_Position (Math|Transform|MakeTransform (- (.location _returnvalue) "0.000000,0.000000,10.000000") (.rotation _returnvalue) (.scale _returnvalue)))
  (Input|EnableInput (Game|GetPlayerController 0)))

(fn ConstructionScript)