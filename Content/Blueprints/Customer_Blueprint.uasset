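; Customer actor that randomly orders an apple pie or water and shows the request on a TextRender.
; While no order is active, each Tick has a small random chance to start one, setting a food or water flag.
; On Hit, a matching Apple_pie_Blueprint or Drop_Blueprint is destroyed and clears the order.
; Water drops are destroyed on contact even without a water order, while pies are only consumed when food is wanted.
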(event EventTick
  (params (DeltaSeconds :type Float%20%28single-precision%29))
  (bind _isasking (CallFunction|IsAsking))
  (if (not _isasking)
    (if (Math|Random|RandomBoolwithWeight 0.001)
      (if (Math|Random|RandomBool)
        (Rendering|Components|TextRender|SetText (Variables|Default|GetTextRender) (Utilities|Text|ToText(String) "One Apple Pie Please"))
        (Variables|Default|SetAskingForFood true)
        (else
          (Rendering|Components|TextRender|SetText (Variables|Default|GetTextRender) (Utilities|Text|ToText(String) "Water Please"))
          (Variables|Default|SetAskingForWater true))))))

(event Collision|EventActorBeginOverlap
  (params (OtherActor :type Actor%20Object%20Reference)))

(event EventBeginPlay
  (Rendering|Components|TextRender|SetText (Variables|Default|GetTextRender) (Utilities|Text|ToText(String) "")))

(event Collision|EventHit
  (params (MyComp :type Primitive%20Component%20Object%20Reference) (Other :type Actor%20Object%20Reference) (OtherComp :type Primitive%20Component%20Object%20Reference) (bSelfMoved :type Boolean) (HitLocation :type Vector :default "0, 0, 0") (HitNormal :type Vector :default "0, 0, 0") (NormalImpulse :type Vector :default "0, 0, 0") (Hit :type Hit%20Result%20Structure%20%28by%20ref%29))
  (bind _returnvalue (Utilities|GetClass Other))
  (if (== _returnvalue "/Game/Blueprints/drop_Blueprint.drop_Blueprint_C")
    (Actor|DestroyActor Other)
    (if (Variables|Default|GetAskingForWater)
      (Rendering|Components|TextRender|SetText (Variables|Default|GetTextRender) (Utilities|Text|ToText(String) ""))
      (Variables|Default|SetAskingForWater false))
    (elif (== _returnvalue "/Game/Blueprints/Apple_pie_Blueprint.Apple_pie_Blueprint_C")
      (if (Variables|Default|GetAskingForFood)
        (Actor|DestroyActor Other)
        (Rendering|Components|TextRender|SetText (Variables|Default|GetTextRender) (Utilities|Text|ToText(String) ""))
        (Variables|Default|SetAskingForFood false)))))

(fn ConstructionScript)

(fn IsAsking
  (return (or (Variables|Default|GetAskingForFood) (Variables|Default|GetAskingForWater))))