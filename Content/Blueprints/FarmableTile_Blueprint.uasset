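; Farm plot actor that grows carrots from seeds and water drops that overlap it.
; A seed is consumed to mark the plot seeded; a drop refills wetness when its overlap ends.
; A one-second timer advances growth and drains wetness while seeded, unfilled and wetness is non-negative.
; Tick turns both progress bars toward the camera and spawns a carrot at full growth, blocking regrowth until that carrot leaves.
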(event EventBeginPlay
  (Variables|Default|SetGrowth 0.0)
  (Utilities|Time|SetTimerbyFunctionName 0 "GrowingPerSec" 1.0 true))

(event Collision|EventActorEndOverlap
  (params (OtherActor :type Actor%20Object%20Reference))
  (if (== OtherActor (Variables|Default|GetCurrCarrot))
    (Variables|Default|SetisFilled false))
  (Utilities|Casting|CastTodrop_Blueprint OtherActor)
  (Variables|Default|SetWetness 1.0))

(event EventTick
  (params (DeltaSeconds :type Float%20%28single-precision%29))
  (CallFunction|UpdateProgress)
  (if (and (Variables|Default|GetisSeeded) (and (not (Variables|Default|GetisFilled)) (>= (Variables|Default|GetWetness) 0.0)))
    (Variables|Default|SetisGrowing true)
    (else
      (Variables|Default|SetisGrowing false)))
  (if (>= (Variables|Default|GetGrowth) 1.0)
    (Utilities|FlowControl|ForLoopwithBreak 0 0
      (:LoopBody
        (bind _returnvalue (Game|SpawnActorfromClass "/Game/Blueprints/carrot_Blueprint.carrot_Blueprint_C" (Math|Transform|MakeTransform (+ (Transformation|GetActorLocation self) "") "-90.000000, 0, 0") "AlwaysSpawn" 0 0))
        (Physics|SetEnableGravity (Variables|/Script/Engine.StaticMeshActor|GetStaticMeshComponent _returnvalue) true)
        (Transformation|SetMobility _returnvalue "Movable")
        (Variables|Default|SetCurrCarrot _returnvalue)
        (Variables|Default|SetisFilled true)
        (Variables|Default|SetisSeeded false))
      (:Completed
        (Variables|Default|SetGrowth 0.0)
        (Audio|PlaySoundatLocation "/Game/Audios/item-receiving.item-receiving" (Transformation|GetActorLocation self) "0, 0, 0" 1.0 1.0 0.0 0 0 0 0)))))

(event Collision|EventActorBeginOverlap
  (params (OtherActor :type Actor%20Object%20Reference))
  (Utilities|Casting|CastToseed_Blueprint OtherActor)
  (Variables|Default|SetisSeeded true)
  (Actor|DestroyActor OtherActor))

(fn ConstructionScript)

(fn GrowingPerSec
  (if (Variables|Default|GetisGrowing)
    (Variables|Default|SetGrowth (+ (Variables|Default|GetGrowth) (Variables|Default|GetGrowingSpeed)))
    (Variables|Default|SetWetness (+ (Variables|Default|GetWetness) -0.01))))

(fn UpdateProgress
  (bind _progressbar (Variables|Default|GetProgressBar))
  (bind _asprogress_bar_widget_blueprint (Utilities|Casting|CastToProgressBarWidgetBlueprint (UserInterface|GetUserWidgetObject (Variables|Default|GetProgressBar))))
  (Default|SetPercent0 _asprogress_bar_widget_blueprint (Variables|Default|GetGrowth))
  (Transformation|SetWorldRotation _progressbar (Math|Rotator|FindLookatRotation (Transformation|GetWorldLocation _progressbar) (Transformation|GetWorldLocation (Variables|/Script/Engine.PlayerCameraManager|GetTransformComponent (Game|GetPlayerCameraManager 0)))) false false)
  (bind _asbackward_progress_bar_widget_blueprint_1 (Utilities|Casting|CastToBackwardProgressBarWidgetBlueprint1 (UserInterface|GetUserWidgetObject (Variables|Default|GetWetnessBar))))
  (Default|SetPercent0 _asbackward_progress_bar_widget_blueprint_1 (Variables|Default|GetWetness)))