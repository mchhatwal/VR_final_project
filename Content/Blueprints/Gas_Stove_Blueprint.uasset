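; Gas stove actor for a restaurant game that shows or removes a flame to match the game state's gas setting.
; Each Tick it polls GasOn on RestaurantGameState, spawning a Fire_Blueprint actor at a hard-coded world location when gas is on and destroying it when off.
; A FireExist flag ensures only one fire is spawned at a time.
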(event EventBeginPlay)

(event EventTick
  (params (DeltaSeconds :type Float%20%28single-precision%29))
  (bind _asrestaurant_game_state (Utilities|Casting|CastToRestaurantGameState (Game|GetGameState)))
  (if (Variables|/Game/Blueprints/RestaurantGameState.RestaurantGameState_C|GetGas_On _asrestaurant_game_state)
    (if (not (Variables|Default|GetFire_Exist))
      (bind _returnvalue (Game|SpawnActorfromClass "/Game/Blueprints/Fire_Blueprint.Fire_Blueprint_C" (Math|Transform|MakeTransform "1160.000000,450.000000,-100.000000") "AlwaysSpawn" 0 0))
      (Variables|Default|SetFire _returnvalue)
      (Variables|Default|SetFire_Exist true)
      (Development|PrintString "FireFireFFFFFFFFFFFFFFFFFFFFFFFFFFFFF" false true "(R=0.000000,G=0.660000,B=1.000000,A=1.000000)" 2e+01))
    (elif (Variables|Default|GetFire_Exist)
      (Actor|DestroyActor (Variables|Default|GetFire))
      (Variables|Default|SetFire_Exist false))))

(fn ConstructionScript)