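; Tree actor that grows over time while it has wetness and spawns a batch of apples when growth completes.
; A one-second looping timer adds growth and drains wetness while growing is allowed.
; Tick checks both values, spawns gravity-free apples at random offsets above the tree, resets growth and plays a sound at world origin.
; It also updates the growth and wetness widget bars, rotating them toward the player camera.
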(event EventBeginPlay
  (Variables|Default|SetGrowth 0.0)
  (Utilities|Time|SetTimerbyFunctionName 0 "GrowingPerSec" 1.0 true))

(event EventTick
  (params (DeltaSeconds :type Float%20%28single-precision%29))
  (CallFunction|UpdateProgress)
  (if (>= (Variables|Default|GetWetness) 0.0)
    (Variables|Default|SetisGrowing true)
    (else
      (Variables|Default|SetisGrowing false)))
  (if (>= (Variables|Default|GetGrowth) 1.0)
    (Utilities|FlowControl|ForLoopwithBreak 0 (Variables|Default|GetnumAppleGrown)
      (:LoopBody
        (bind _returnvalue (Game|SpawnActorfromClass "/Game/Blueprints/BP_Apple.BP_Apple_C" (Math|Conversions|ToTransform(Vector) (+ (+ (Transformation|GetActorLocation self) (* (Math|Random|RandomUnitVector) (- (* (Class|KismetMathLibrary|VectorOne) "200.000000,200.000000,200.000000") "100.000000,100.000000,100.000000"))) "0,0,200.000000")) "AdjustIfPossibleButAlwaysSpawn" 0 0))
        (Physics|SetEnableGravity (Variables|/Script/Engine.StaticMeshActor|GetStaticMeshComponent _returnvalue) false)
        (Transformation|SetMobility _returnvalue "Movable"))
      (:Completed
        (Variables|Default|SetGrowth 0.0)
        (Audio|PlaySoundatLocation "/Game/Audios/item-receiving.item-receiving" "0, 0, 0" "0, 0, 0" 1.0 1.0 0.0 0 0 0 0)))))

(event Collision|EventActorBeginOverlap
  (params (OtherActor :type Actor%20Object%20Reference)))

(fn ConstructionScript)

(fn GrowingPerSec
  (if (Variables|Default|GetisGrowing)
    (Variables|Default|SetGrowth (+ (Variables|Default|GetGrowth) (Variables|Default|GetGrowingSpeed)))
    (Variables|Default|SetWetness (+ (Variables|Default|GetWetness) -0.01))))

(fn UpdateProgress
  (bind _progressbar (Variables|Default|GetProgressBar))
  (bind _asprogress_bar_widget_blueprint (Utilities|Casting|CastToProgressBarWidgetBlueprint (UserInterface|GetUserWidgetObject (Variables|Default|GetProgressBar))))
  (Default|SetPercent0 _asprogress_bar_widget_blueprint (Variables|Default|GetGrowth))
  (Transformation|SetWorldRotation _progressbar (Math|Rotator|FindLookatRotation (Transformation|GetWorldLocation _progressbar) (Transformation|GetWorldLocation (Variables|/Script/Engine.PlayerCameraManager|GetTransformComponent (Game|GetPlayerCameraManager 0)))) false false)
  (bind _asbackward_progress_bar_widget_blueprint_1 (Utilities|Casting|CastToBackwardProgressBarWidgetBlueprint1 (UserInterface|GetUserWidgetObject (Variables|Default|GetWetnessBar))))
  (Default|SetPercent0 _asbackward_progress_bar_widget_blueprint_1 (Variables|Default|GetWetness)))