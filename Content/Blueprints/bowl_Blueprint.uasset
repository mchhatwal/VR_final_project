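; Mixing bowl actor that collects water, flour and sliced apple, then produces a raw apple pie.
; On Hit, exact class checks treat drops as water, spheres as flour and sliced apple as apple, setting a flag and destroying that actor.
; Tick polls the three flags and, once all are set, spawns one BP_Pie_Raw at a hard-coded world location with the bowl's rotation, guarded against repeats.
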(event EventBeginPlay)

(event Collision|EventActorBeginOverlap
  (params (OtherActor :type Actor%20Object%20Reference)))

(event EventTick
  (params (DeltaSeconds :type Float%20%28single-precision%29))
  (if (Math|Boolean|ANDBoolean (Variables|Default|Gethas_water) (Variables|Default|Gethas_apple) (Variables|Default|Gethas_flour))
    (if (not (Variables|Default|Gethas_sapwn_pie))
      (Game|SpawnActorfromClass "/Game/Blueprints/BP_Pie_Raw.BP_Pie_Raw_C" (Math|Transform|MakeTransform (Math|Vector|MakeVector 1.12e+03 9e+01 9e+01) (.Rotation (Math|Transform|BreakTransform (Transformation|GetActorTransform))) "0.500000,0.500000,0.500000") "Undefined" 0 0)
      (Variables|Default|Sethas_sapwn_pie true))))

(event Collision|EventHit
  (params (MyComp :type Primitive%20Component%20Object%20Reference) (Other :type Actor%20Object%20Reference) (OtherComp :type Primitive%20Component%20Object%20Reference) (bSelfMoved :type Boolean) (HitLocation :type Vector :default "0, 0, 0") (HitNormal :type Vector :default "0, 0, 0") (NormalImpulse :type Vector :default "0, 0, 0") (Hit :type Hit%20Result%20Structure%20%28by%20ref%29))
  (bind _returnvalue (Utilities|GetClass Other))
  (Development|PrintString "hit happen" false)
  (if (== _returnvalue "/Game/Blueprints/drop_Blueprint.drop_Blueprint_C")
    (Variables|Default|Sethas_water true)
    (Development|PrintString "water true" false)
    (Actor|DestroyActor Other :!label _label)
    (elif (== _returnvalue "/Game/Blueprints/Sphere_Blueprint.Sphere_Blueprint_C")
      (Variables|Default|Sethas_flour true)
      (Development|PrintString "flour true" false)
      (goto _label)
      (elif (== _returnvalue "/Game/Blueprints/Sliced_Apple_Blueprint.Sliced_Apple_Blueprint_C")
        (Variables|Default|Sethas_apple true)
        (Development|PrintString "apple true" false)
        (goto _label)))))

(fn ConstructionScript)