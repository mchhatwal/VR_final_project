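; Carrot actor that can be grabbed and sold for money at a sell box.
; When grabbed through its Grab component, it sets its static mesh to a fixed small world scale.
; Hitting a Sellbox_Blueprint adds a fixed amount to Money on every Shop_manager_Blueprint found in the level, then destroys the carrot.
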(event OnGrabbed(Grab)
  (Transformation|SetWorldScale3D (Variables|Debug|GetStaticMeshComponent) "0.050000,0.050000,0.050000"))

(event EventBeginPlay)

(event Collision|EventActorBeginOverlap
  (params (OtherActor :type Actor%20Object%20Reference)))

(event EventTick
  (params (DeltaSeconds :type Float%20%28single-precision%29)))

(event Collision|EventHit
  (params (MyComp :type Primitive%20Component%20Object%20Reference) (Other :type Actor%20Object%20Reference) (OtherComp :type Primitive%20Component%20Object%20Reference) (bSelfMoved :type Boolean) (HitLocation :type Vector :default "0, 0, 0") (HitNormal :type Vector :default "0, 0, 0") (NormalImpulse :type Vector :default "0, 0, 0") (Hit :type Hit%20Result%20Structure%20%28by%20ref%29))
  (if (== (Utilities|GetClass Other) "/Game/Blueprints/sellbox_Blueprint.sellbox_Blueprint_C")
    (bind _outactors (Actor|GetAllActorsOfClass "/Game/Blueprints/shop_manager_Blueprint.shop_manager_Blueprint_C"))
    (for _array_element _outactors
      (Variables|/Game/Blueprints/shop_manager_Blueprint.shop_manager_Blueprint_C|Setmoney _array_element (+ (Variables|/Game/Blueprints/shop_manager_Blueprint.shop_manager_Blueprint_C|Getmoney _array_element) 3)))
    (Actor|DestroyActor)))

(fn ConstructionScript)