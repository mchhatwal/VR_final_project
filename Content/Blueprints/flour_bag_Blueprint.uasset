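; Flour bag actor that pours out flour, represented by small sphere actors, when its roll leaves a set range.
; Each Tick it reads the GrabComponent's world roll and treats values outside the 45 to 135 degree band as tipped.
; While tipped, it spawns a scaled-down Sphere_Blueprint just below itself every frame, with no timer or spawn limit.
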(event EventBeginPlay)

(event Collision|EventActorBeginOverlap
  (params (OtherActor :type Actor%20Object%20Reference)))

(event EventTick
  (params (DeltaSeconds :type Float%20%28single-precision%29))
  (bind _grabcomponent (Variables|Default|GetGrabComponent))
  (bind _returnvalue (Transformation|GetWorldRotation _grabcomponent))
  (bind _roll (Math|Rotator|BreakRotator _returnvalue))
  (if (or (> _roll 135.0) (< _roll 45.0))
    (Game|SpawnActorfromClass "/Game/Blueprints/Sphere_Blueprint.Sphere_Blueprint_C" (Math|Transform|MakeTransform (+ (Transformation|GetActorLocation) "0,0,-25.000000") (Transformation|GetActorRotation) "0.300000,0.300000,0.300000") "Undefined" 0 0)))

(fn ConstructionScript)