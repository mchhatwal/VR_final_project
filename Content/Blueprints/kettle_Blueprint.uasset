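; Kettle actor that pours liquid when tilted by spawning Drop_Blueprint actors.
; Tick accumulates delta time and, at a short fixed interval, checks the world pitch of its static mesh component.
; While the pitch is within the forward tilt range, it spawns one drop per interval at the actor's own transform.
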(event EventBeginPlay)

(event Collision|EventActorBeginOverlap
  (params (OtherActor :type Actor%20Object%20Reference)))

(event EventTick
  (params (DeltaSeconds :type Float%20%28single-precision%29))
  (bind _staticmeshcomponent (Variables|Debug|GetStaticMeshComponent))
  (bind _returnvalue (Transformation|GetWorldRotation _staticmeshcomponent))
  (bind _pitch (Math|Rotator|BreakRotator _returnvalue))
  (bind _output_get (Variables|Default|SetLastSpawn (+ DeltaSeconds (Variables|Default|GetLastSpawn))))
  (if (>= _output_get 0.1)
    (Variables|Default|SetLastSpawn 0.0)
    (if (and (>= _pitch 45.0) (<= _pitch 9e+01))
      (Game|SpawnActorfromClass "/Game/Blueprints/drop_Blueprint.drop_Blueprint_C" (Transformation|GetActorTransform) "Undefined" 0 0))))

(fn ConstructionScript)