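; Sofa-table actor that acts as a selling point for finished pies in a shop game.
; When hit by a BP_Pie_Done, it marks every unsold pie in the level as sold, not just the one that hit.
; Each sale adds money to the Shop_manager_Blueprint found by class search.
; It also spawns an Add_money_Blueprint above the pie returned by GetActorOfClass, rotated toward the player.
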(event EventBeginPlay)

(event Collision|EventActorBeginOverlap
  (params (OtherActor :type Actor%20Object%20Reference)))

(event EventTick
  (params (DeltaSeconds :type Float%20%28single-precision%29)))

(event Collision|EventHit
  (params (MyComp :type Primitive%20Component%20Object%20Reference) (Other :type Actor%20Object%20Reference) (OtherComp :type Primitive%20Component%20Object%20Reference) (bSelfMoved :type Boolean) (HitLocation :type Vector :default "0, 0, 0") (HitNormal :type Vector :default "0, 0, 0") (NormalImpulse :type Vector :default "0, 0, 0") (Hit :type Hit%20Result%20Structure%20%28by%20ref%29))
  (if (== (Utilities|GetClass Other) "/Game/Blueprints/BP_Pie_Done.BP_Pie_Done_C")
    (bind _outactors (Actor|GetAllActorsOfClass "/Game/Blueprints/BP_Pie_Done.BP_Pie_Done_C"))
    (for _array_element _outactors
      (if (not (Variables|/Game/Blueprints/BP_Pie_Done.BP_Pie_Done_C|Getselled _array_element))
        (Variables|/Game/Blueprints/BP_Pie_Done.BP_Pie_Done_C|Setselled _array_element true)
        (bind _outactors_2 (Actor|GetAllActorsOfClass "/Game/Blueprints/shop_manager_Blueprint.shop_manager_Blueprint_C"))
        (for _array_element_2 _outactors_2
          (Variables|/Game/Blueprints/shop_manager_Blueprint.shop_manager_Blueprint_C|Setmoney _array_element_2 (+ (Variables|/Game/Blueprints/shop_manager_Blueprint.shop_manager_Blueprint_C|Getmoney _array_element_2) 10))
          (bind _returnvalue (Actor|GetActorOfClass "/Game/Blueprints/BP_Pie_Done.BP_Pie_Done_C"))
          (Game|SpawnActorfromClass "/Game/Blueprints/add_money_Blueprint.add_money_Blueprint_C" (Math|Transform|MakeTransform (+ (.Location (Math|Transform|BreakTransform (Transformation|GetActorTransform _returnvalue))) "0,0,20.000000") (Math|Rotator|FindLookatRotation (+ (.Location (Math|Transform|BreakTransform (Transformation|GetActorTransform _returnvalue))) "0,0,20.000000") (Transformation|GetActorLocation (Game|Player|GetPlayerPawn 0)))) "Undefined" 0 0))))))

(fn ConstructionScript)